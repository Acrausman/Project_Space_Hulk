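; A double glass door actor that opens automatically when something overlaps its Box and closes when the overlap ends.
; Each overlap event waits a short delay, then plays or reverses two Timelines, one per door mesh.
; The Timelines lerp the meshes' relative locations in opposite directions along X to slide the panels, with no filter on the overlapping actor.
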(event OnComponentEndOverlap(Box)
  (params (OverlappedComponent :type Primitive%20Component%20Object%20Reference) (OtherActor :type Actor%20Object%20Reference) (OtherComp :type Primitive%20Component%20Object%20Reference) (OtherBodyIndex :type Integer))
  (Utilities|FlowControl|Delay 1.0)
  (Utilities|FlowControl|Sequence
    (:then_0
      (bind _newtrack_0 (Timeline|Timeline_0 Reverse)
        (:Update
          (Transformation|SetRelativeLocation (Variables|Default|GetStaticMesh) (Math|Vector|Lerp(Vector) "350.000000,-250.000000,-40.000000" "0.000000,-250.000000,-40.000000" _newtrack_0) false false))))
    (:then_1
      (bind _newtrack_0_2 (Timeline|Timeline_1 Reverse)
        (:Update
          (Transformation|SetRelativeLocation (Variables|Default|GetStaticMesh1) (Math|Vector|Lerp(Vector) "295.000000,240.000000,-40.000000" "645.000000,240.000000,-40.000000" _newtrack_0_2) false false))))))

(event OnComponentBeginOverlap(Box)
  (params (OverlappedComponent :type Primitive%20Component%20Object%20Reference) (OtherActor :type Actor%20Object%20Reference) (OtherComp :type Primitive%20Component%20Object%20Reference) (OtherBodyIndex :type Integer) (bFromSweep :type Boolean) (SweepResult :type Hit%20Result%20Structure%20%28by%20ref%29))
  (Utilities|FlowControl|Delay 1.0)
  (Utilities|FlowControl|Sequence
    (:then_0
      (bind _newtrack_0 (Timeline|Timeline_0 Play)
        (:Update
          (Transformation|SetRelativeLocation (Variables|Default|GetStaticMesh) (Math|Vector|Lerp(Vector) "350.000000,-250.000000,-40.000000" "0.000000,-250.000000,-40.000000" _newtrack_0) false false))))
    (:then_1
      (bind _newtrack_0_2 (Timeline|Timeline_1 Play)
        (:Update
          (Transformation|SetRelativeLocation (Variables|Default|GetStaticMesh1) (Math|Vector|Lerp(Vector) "295.000000,240.000000,-40.000000" "645.000000,240.000000,-40.000000" _newtrack_0_2) false false))))))

(fn ConstructionScript)