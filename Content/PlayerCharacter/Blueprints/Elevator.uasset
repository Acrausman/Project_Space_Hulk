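; Elevator actor that carries its static mesh between a lower and upper height when the first-person character enters its box trigger.
; Entering plays or reverses a timeline based on ElevatorIsUp, lerping the mesh's relative location between two hardcoded points without sweep.
; The state flag flips whenever any actor leaves the box, without a character check or waiting for the movement to finish.
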(event OnComponentBeginOverlap(Box)
  (params (OverlappedComponent :type Primitive%20Component%20Object%20Reference) (OtherActor :type Actor%20Object%20Reference) (OtherComp :type Primitive%20Component%20Object%20Reference) (OtherBodyIndex :type Integer) (bFromSweep :type Boolean) (SweepResult :type Hit%20Result%20Structure%20%28by%20ref%29))
  (Utilities|Casting|CastToFirstPersonCharacter OtherActor)
  (if (Variables|Default|Getelevator%20is%20up)
    (bind _newtrack_0 (Timeline|Timeline_0 Reverse)
      (:Update
        (Transformation|SetRelativeLocation (Variables|Default|GetStaticMesh) (Math|Vector|Lerp(Vector) "-10.000000,-20.000000,-80.000000" "-10.000000,-20.000000,5530.000000" _newtrack_0) false false)))
    (else
      (Timeline|Timeline_0 Play))))

(event OnComponentEndOverlap(Box)
  (params (OverlappedComponent :type Primitive%20Component%20Object%20Reference) (OtherActor :type Actor%20Object%20Reference) (OtherComp :type Primitive%20Component%20Object%20Reference) (OtherBodyIndex :type Integer))
  (if (Variables|Default|Getelevator%20is%20up)
    (Variables|Default|Setelevator%20is%20up false)
    (else
      (Variables|Default|Setelevator%20is%20up true))))

(fn ConstructionScript)